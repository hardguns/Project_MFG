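; Gameplay player controller that starts in game-only input and opens the pause menu.
; On the Pause input it creates and displays a new pause menu widget, then hides the MFG_Character's main HUD if visible.
; It then switches to UI-only input with an unlocked mouse and visible cursor.
; It does not pause the game or handle resuming itself.
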(event `self.ReceiveBeginPlay`
  (`WidgetBlueprintLibrary.SetInputMode_GameOnly` self))

(event `InputAction|Pause` :paused true
  (params (Key :type "Key Structure"))
  (:`Pressed`
    (`|ExecutionSequence`
      (:`then_0`
        (bind _returnvalue (`|CreateWidget` "/Game/Blueprints/UI/PauseMenu/W_PauseMenuWidget.W_PauseMenuWidget_C"))
        (bind _output_get (set `self.PauseMenuRef` _returnvalue))
        (`UserWidget.AddToViewport` _output_get 0)
        (bind _asmfg_character (cast `MFG_Character` (`GameplayStatics.GetPlayerCharacter` 0)))
        (bind _charactermainhud (`MFG_Character.CharacterMainHUD` _asmfg_character))
        (if (`Widget.IsVisible` _charactermainhud)
          (`Widget.SetVisibility` _charactermainhud "Hidden")))
      (:`then_1`
        (`WidgetBlueprintLibrary.SetInputMode_UIOnlyEx` self null)
        (set `self.bShowMouseCursor` true)))))

(fn `UserConstructionScript`)