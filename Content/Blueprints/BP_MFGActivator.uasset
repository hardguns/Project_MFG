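; BP_MFGActivator is an activator actor whose PointLight shows the value of its SwitchState flag as green for true and red for false.
; BeginPlay sets the initial light color from that flag.
; The UseActivator event prints a debug message and reapplies the same color check, without changing SwitchState itself.
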(event `self.ReceiveBeginPlay`
  (bind _pointlight (`self.PointLight`))
  (if (`self.bSwitchState`)
    (`LightComponent.SetLightColor` _pointlight (struct :`R` 0.009047 :`G` 0.328125 :`A` 1.0) true)
    (else
      (`LightComponent.SetLightColor` _pointlight (struct :`R` 0.489583 :`A` 1.0) true))))

(event `self.BP_UseActivator`
  (bind _pointlight (`self.PointLight`))
  (`KismetSystemLibrary.PrintString` "Activator has been used" true true (struct :`R` 1.0 :`G` 0.088762 :`A` 1.0) 3.0)
  (if (`self.bSwitchState`)
    (`LightComponent.SetLightColor` _pointlight (struct :`R` 0.009047 :`G` 0.328125 :`A` 1.0) true)
    (else
      (`LightComponent.SetLightColor` _pointlight (struct :`R` 0.489583 :`A` 1.0) true))))

(fn `UserConstructionScript`)