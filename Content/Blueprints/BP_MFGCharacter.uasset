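; Player character Blueprint that creates the main HUD, shows objectives while an input is held, and selects first- or third-person camera at construction.
; Ultimate start and stop swap post-process settings; key 1 grants ultimate XP.
; Sight collider overlaps run a looping timer that sphere-scans and line-traces to enemies, setting their "seen by player" blackboard flag unless an Obstacle-tagged actor blocks.
; End overlap stops the timer and clears that enemy's flag.
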(event `self.ReceiveBeginPlay`
  (`|ExecutionSequence`
    (:`then_0`
      (bind _returnvalue (`|CreateWidget` "/Game/Blueprints/UI/HUD/W_MainHUD.W_MainHUD_C"))
      (bind _output_get (set `self.CharacterMainHUD` _returnvalue))
      (`UserWidget.AddToViewport` _output_get 0))
    (:`then_1`
      (set `self.NormalPostProcess` (`PostProcessComponent.Settings` (`self.PostProcess`))))))

(event `self.ReceiveAnyDamage`
  (params (Damage :type "Float (single-precision)") (DamageType :type "DamageType Object Reference") (InstigatedBy :type "Controller Object Reference") (DamageCauser :type "Actor Object Reference")))

(event `self.BP_StartUltimate`
  (set `PostProcessComponent.Settings` (make `PostProcessSettings` :`WhiteTemp` 10000.0 :`FilmSlope` 1.2 :`FilmBlackClip` 0.02) (`self.PostProcess`)))

(event `self.BP_StopUltimate`
  (set `PostProcessComponent.Settings` (`self.NormalPostProcess`) (`self.PostProcess`)))

(event `self.SightCollider.OnComponentBeginOverlap`
  (params (OverlappedComponent :type "PrimitiveComponent Object Reference") (OtherActor :type "Actor Object Reference") (OtherComp :type "PrimitiveComponent Object Reference") (OtherBodyIndex :type Integer) (bFromSweep :type Boolean) (SweepResult :type "HitResult Structure (by ref)"))
  (if (not (`MFG_HealthComponent.IsDead` (`self.HealthComponent`)))
    (bind _returnvalue (`KismetSystemLibrary.K2_SetTimer` null "UpdateLookForEnemy" 0.5 true))))

(event `self.SightCollider.OnComponentEndOverlap`
  (params (OverlappedComponent :type "PrimitiveComponent Object Reference") (OtherActor :type "Actor Object Reference") (OtherComp :type "PrimitiveComponent Object Reference") (OtherBodyIndex :type Integer))
  (`KismetSystemLibrary.K2_ClearAndInvalidateTimerHandle` (stale `self.SightCollider.OnComponentBeginOverlap` _returnvalue))
  (bind _asmfg_character (cast `MFG_Character` OtherActor))
  (bind _returnvalue (`self.GetCharacterType` _asmfg_character))
  (if (`|EnumEquality` _returnvalue "CharacterType_Enemy")
    (bind _returnvalue_2 (`AIBlueprintHelperLibrary.GetBlackboard` _asmfg_character))
    (`/Engine/EditorBlueprintResources/StandardMacros.IsValid` _returnvalue_2
      (:`Is Valid`
        (`BlackboardComponent.SetValueAsBool` _returnvalue_2 "bIsBeingSeeingByPlayer" false)))))

(event `self.BP_UpdateUltimateDuration`
  (params (Value :type "Float (single-precision)")))

(event `self.BP_GainUltimateXP`
  (params (XPGained :type "Float (single-precision)")))

(event `InputAction|ObjectivesPanel`
  (params (Key :type "Key Structure"))
  (:`Pressed`
    (bind _asw_main_hud (cast `/Game/Blueprints/UI/HUD/W_MainHUD` (`self.CharacterMainHUD`)))
    (`Widget.SetVisibility` (`/Game/Blueprints/UI/HUD/W_MainHUD.W_ObjectivesContainer` _asw_main_hud) "Visible"))
  (:`Released`
    (bind _asw_main_hud_2 (cast `/Game/Blueprints/UI/HUD/W_MainHUD` (`self.CharacterMainHUD`)))
    (`Widget.SetVisibility` (`/Game/Blueprints/UI/HUD/W_MainHUD.W_ObjectivesContainer` _asw_main_hud_2) "Hidden")))

(event `Key|One`
  (params (Key :type "Key Structure"))
  (:`Pressed`
    (`self.GainUltimateXP` 1000.0)))

(fn `UpdateLookForEnemy`
  (`KismetSystemLibrary.PrintString` "Executing UpdateEnemySeen" false false (struct :`R` 0.151363 :`G` 0.038445 :`B` 1.0 :`A` 1.0))
  (bind _outactors (`KismetSystemLibrary.SphereOverlapActors` (`self.K2_GetActorLocation`) 1000.0 (`|MakeArray` "ObjectTypeQuery7" :!type "EObjectTypeQuery Enum")))
  (for _array_element _outactors
    (bind _outhit (`KismetSystemLibrary.LineTraceSingleForObjects` (`self.K2_GetActorLocation`) (`self.K2_GetActorLocation` _array_element) (`|MakeArray` "ObjectTypeQuery1" "ObjectTypeQuery7" :!type "EObjectTypeQuery Enum")))
    (bind _asmfg_enemy (cast `MFG_Enemy` _array_element))
    (bind _returnvalue (`AIBlueprintHelperLibrary.GetBlackboard` _asmfg_enemy))
    (`/Engine/EditorBlueprintResources/StandardMacros.IsValid` _returnvalue
      (:`Is Valid`
        (`BlackboardComponent.SetValueAsBool` _returnvalue "bIsBeingSeeingByPlayer" (not (`self.ActorHasTag` (`.HitActor` (`GameplayStatics.BreakHitResult` _outhit)) "Obstacle")))))))

(fn `UserConstructionScript`
  (`ActorComponent.SetAutoActivate` (`self.FPSCameraComponent`) (`self.bUseFirstPersonView`))
  (`ActorComponent.SetAutoActivate` (`self.SpringArmComponent`) (not (`self.bUseFirstPersonView`)))
  (`ActorComponent.SetAutoActivate` (`self.TPSCameraComponent`) (not (`self.bUseFirstPersonView`))))