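; BP_Enemy is an enemy AI Blueprint whose only live logic prints incoming damage from AnyDamage.
; Its BeginPlay and health-change events are empty.
; Disconnected logic would cache the AIC_Enemy controller and, on death, unpossess and destroy the actor after a delay.
; For non-lethal weapon hits, that unused logic would flag the controller and report an AI damage-sense event from the weapon owner's location.
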(event `self.HealthComponent.OnHealthChangeDelegate`
  (params (HealthComponent :type "MFG_HealthComponent Object Reference") (DamagedActor :type "Actor Object Reference") (Damage :type "Float (single-precision)") (DamageType :type "DamageType Object Reference") (InstigatedBy :type "Controller Object Reference") (DamageCauser :type "Actor Object Reference")))

(event `self.ReceiveBeginPlay`)

(event `self.ReceiveAnyDamage`
  (params (Damage :type "Float (single-precision)") (DamageType :type "DamageType Object Reference") (InstigatedBy :type "Controller Object Reference") (DamageCauser :type "Actor Object Reference"))
  (`KismetSystemLibrary.PrintString` (`KismetStringLibrary.Conv_DoubleToString` Damage)))

(fn `UserConstructionScript`)