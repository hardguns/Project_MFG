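; AIC_Enemy is an enemy AI controller with an AIPerception component, but its Blueprint logic is disconnected, so its events do nothing.
; Unwired nodes would run BT_EnemyFCAttacking and copy MFG_Enemy patrol settings to the Blackboard.
; Other unwired chains would filter perceived characters to players and write sight and damage-investigation keys, assuming stimulus index 0 is sight and 1 is damage.
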(event `self.ReceiveBeginPlay`)

(event `self.AIPerception.OnTargetPerceptionUpdated`
  (params (Actor :type "Actor Object Reference") (Stimulus :type "AIStimulus Structure")))

(event `self.AIPerception.OnPerceptionUpdated`
  (params (UpdatedActors :type "Array of Actor Object Reference (by ref)")))

(fn `UserConstructionScript`)